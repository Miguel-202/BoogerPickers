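; Windmill puzzle Blueprint that powers a linked door when hit by an Air spell, usable only once.
; The construction script runs a cable spline and spline mesh from the rotor to the door's left panel.
; On activation, Tick moves an electricity effect along the spline.
; At the end, it destroys that effect, signals the door, spawns lightning at the rotor and plays a rotation timeline.
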(event `self.ReceiveBeginPlay`
  ;[1 1 1] Set the points in the spline from the constructor
  (`SplineComponent.SetSplinePoints` (`self.Cable`) (`self.CablePoints`) "World" true))

(event `self.ReceiveTick`
  (params (DeltaSeconds :type "Float (single-precision)"))
  (`self.MoveElectricityParticle` DeltaSeconds))

(event `self.OnInteractedWithSpell`
  (params (spellType :type "ESpellEffects Enum" :default "Fire"))
  ;[1 1 1] Set reactivity to wind spell
  (if (`self.IsActive`)
    _
    (elif (not (`self.HasBeenUsed`))
      (switch `ESpellEffects` spellType
        (:`Air`
          (set `self.IsActive` true))))))

(event `PowerUpDoor`
  (bind _windrotator (`self.WindRotator`))
  (bind (_returnvalue_location _returnvalue_rotation _returnvalue_scale) (`KismetMathLibrary.BreakTransform` (`SceneComponent.K2_GetComponentToWorld` _windrotator)))
  ;[1 1 1] Send Signal to the Door BP to open, and set the wind mill to rotate with WindMillRunning Timeline
  (message `/Game/Blockouts/BPI_ElectricActivity.IsActiveWithElectricity` (`self.Door`) true)
  (`GameplayStatics.SpawnEmitterAtLocation` "/Game/ImportedAssets/Luos8Elements/Particles/Lightning/Par_4E_LightningStrike_01.Par_4E_LightningStrike_01" _returnvalue_location _returnvalue_rotation _returnvalue_scale)
  (bind (_direction _rotation) (`Timeline|WindMillRunning`)
    (:`Update`
      (`SceneComponent.K2_SetWorldTransform` _windrotator (`KismetMathLibrary.MakeTransform` _returnvalue_location (`KismetMathLibrary.MakeRotator` 0.0 (+ _rotation 30.0)) _returnvalue_scale) false false))))

(event `MoveElectricityParticle`
  (params (DeltaTime :type "Float (double-precision)"))
  (bind _electricitytroughcable (`self.ElectricityTroughCable`))
  (bind (_returnvalue_location _returnvalue_rotation) (`KismetMathLibrary.BreakTransform` (`SplineComponent.GetTransformAtDistanceAlongSpline` (`self.Cable`) (`self.CableDistance`) "Local" false)))
  ;[1 1 1] If Active, the Distance will travle trough the spline position at the Electricity speed
  (if (`self.IsActive`)
    (set `self.CableDistance` (+ (* DeltaTime (`self.ElectricitySpeed`)) (`self.CableDistance`)))
    ;[1 1 1] Set the position of the particle effects to the distance inside the spline
    (`SceneComponent.K2_SetRelativeTransform` _electricitytroughcable (`KismetMathLibrary.MakeTransform` _returnvalue_location _returnvalue_rotation (`SceneComponent.RelativeScale3D` _electricitytroughcable)) false false)
    ;[1 1 1] Once it reaches the end, power up the door and make sure to set it Has ben used so you can't trigger it twice
    (if (>= (`self.CableDistance`) (`SplineComponent.GetSplineLength` (`self.Cable`)))
      (`ActorComponent.K2_DestroyComponent` (`self.ElectricityTroughCable`))
      (`self.PowerUpDoor`)
      (set `self.IsActive` false)
      (set `self.HasBeenUsed` true))))

(fn `UserConstructionScript`
  (bind _cablepoints (`self.CablePoints`))
  (bind _splinemesh (`self.SplineMesh`))
  (bind _returnvalue (`SceneComponent.K2_GetComponentLocation` (`self.WindRotator`)))
  (bind _returnvalue_2 (`SceneComponent.K2_GetComponentLocation` (`/Game/Blockouts/BP_WindPoweredDoor.DoorLeft` (`self.Door`))))
  (set `self.IsActive` false)
  (`KismetArrayLibrary.Array_Add` _cablepoints _returnvalue)
  (`KismetArrayLibrary.Array_Add` _cablepoints _returnvalue_2)
  ;[1 1 1] After setting the spline points, now set the SplineMesh points
  (`SplineMeshComponent.SetEndPosition` _splinemesh _returnvalue_2 true)
  (`SplineMeshComponent.SetStartPosition` _splinemesh _returnvalue true)
  (set `self.HasBeenUsed` false))