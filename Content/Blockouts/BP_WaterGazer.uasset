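; BP_WaterGazer is a blockout water geyser that fire and ice spells toggle between flowing and frozen.
; Melted, it shows particles, overlaps pawns, and plays the GazerUp timeline to scale particles, ice mesh and collision box together.
; Frozen, it shows ice, blocks pawns and stops the timeline, holding the current height.
; The construction script clears IsFrozen, so BeginPlay normally starts it melted.
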(event `self.ReceiveBeginPlay`
  (if (`self.IsFrozen`)
    (`self.FreezeGazer`)
    (else
      (`self.MeltGazer`))))

(event `self.OnInteractedWithSpell`
  (params (spellType :type "ESpellEffects Enum" :default "Fire"))
  (switch `ESpellEffects` spellType
    (:`Fire`
      (if (`self.IsFrozen`)
        (`self.MeltGazer`)))
    (:`Ice`
      (if (not (`self.IsFrozen`))
        (`self.FreezeGazer`)))))

(event `MeltGazer`
  (`SceneComponent.SetVisibility` (`self.ParticleSystem`) true true)
  (`SceneComponent.SetVisibility` (`self.Ice1`) false true)
  (set `self.IsFrozen` false)
  (`PrimitiveComponent.SetCollisionResponseToChannel` (`self.BoxCollision`) "ECC_Pawn" "ECR_Overlap")
  (bind (_direction _gazerheight) (`Timeline|GazerUp` :!label _label)
    (:`Update`
      (`SceneComponent.SetWorldScale3D` (`self.Ice1`) (* (3.5 1.25 1.25) _gazerheight))
      (`SceneComponent.SetWorldScale3D` (`self.ParticleSystem`) (* (0.2 0.2 2.0) _gazerheight))
      (`SceneComponent.SetWorldScale3D` (`self.BoxCollision`) (* (1.0 1.0 2.3) _gazerheight)))))

(event `FreezeGazer`
  (`SceneComponent.SetVisibility` (`self.ParticleSystem`) false true)
  (`SceneComponent.SetVisibility` (`self.Ice1`) true true)
  (set `self.IsFrozen` true)
  (`PrimitiveComponent.SetCollisionResponseToChannel` (`self.BoxCollision`) "ECC_Pawn" "ECR_Block")
  (goto _label :!via `Stop`))

(fn `UserConstructionScript`
  (set `self.IsFrozen` false))